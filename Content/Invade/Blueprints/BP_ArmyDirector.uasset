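; BP_ArmyDirector draws curved direction meshes from each land in LandRef to a shared TargetPos, apparently as army movement indicators.
; UpdateArmyDirector, with no caller in this file, grows a reusable spline mesh pool as needed, hides it, then shows one per land.
; Tangents and up vector follow the normalized sum of both positions, arching away from world origin, scaled by distance.
; Each mesh's material receives that distance as Length.
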(fn `HandleSplineMeshInit`
  (params (Count :type Integer))
  (bind _returnvalue (`KismetArrayLibrary.Array_Length` (`self.SplineMeshArray`)))
  (`|ExecutionSequence`
    (:`then_0`
      (if (not (>= _returnvalue Count))
        (for _ (range (- Count _returnvalue))
          (bind _returnvalue_2 (`AddComponent|NODE_AddSplineMeshComponent-2`))
          (`StaticMeshComponent.SetStaticMesh` _returnvalue_2 "/Game/Invade/Meshes/DirMesh.DirMesh")
          (`KismetArrayLibrary.Array_AddUnique` (`self.SplineMeshArray`) _returnvalue_2))))
    (:`then_1`
      (for _array_element (`self.SplineMeshArray`)
        (`SceneComponent.SetVisibility` _array_element false false)))))

(fn `UpdateArmyDirector`
  (bind _targetpos (`self.TargetPos`))
  (`self.HandleSplineMeshInit` (`KismetArrayLibrary.Array_Length` (`self.LandRef`)))
  (for (_array_element _array_index) (`self.LandRef`)
    (bind _output (`|GetArrayItem` (`self.SplineMeshArray`) _array_index))
    (`SceneComponent.SetVisibility` _output true false)
    (bind _returnvalue (`self.K2_GetActorLocation` _array_element))
    (`SplineMeshComponent.SetStartPosition` _output _returnvalue false)
    (bind _returnvalue_2 (`KismetMathLibrary.Normal` (+ _returnvalue _targetpos)))
    (bind _returnvalue_3 (`KismetMathLibrary.Vector_Distance` _returnvalue _targetpos))
    (bind _returnvalue_4 (* _returnvalue_2 (* _returnvalue_3 0.8)))
    (`SplineMeshComponent.SetStartTangent` _output _returnvalue_4 false)
    (`SplineMeshComponent.SetEndPosition` _output _targetpos false)
    (`SplineMeshComponent.SetEndTangent` _output (* _returnvalue_4 -1.0) false)
    (`SplineMeshComponent.SetSplineUpDir` _output _returnvalue_2 true)
    (`MeshComponent.SetScalarParameterValueOnMaterials` _output "Length" _returnvalue_3)))

(fn `UserConstructionScript`)