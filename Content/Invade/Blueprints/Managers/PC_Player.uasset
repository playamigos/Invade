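; Player controller that handles mouse-tap land selection for an army-based game.
; On tap start, it traces under the cursor for a BP_Land and checks whether any army there matches the player state's PlayerIndex.
; Selection results are only debug prints so far.
; Each tap start, cancel and completion resets a BP_ArmyDirector, spawning it if missing and clearing its land references.
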(event `EnhancedInput|/Game/Invade/Input/Actions/IA_MouseTap`
  (params (ActionValue :type Boolean) (ElapsedSeconds :type "Float (double-precision)") (TriggeredSeconds :type "Float (double-precision)") (InputAction :type "InputAction Object Reference" :default "/Game/Invade/Input/Actions/IA_MouseTap.IA_MouseTap"))
  (bind (_locationx _locationy) (`self.GetMousePosition`))
  (bind (_worldlocation _worlddirection) (`self.DeprojectScreenPositionToWorld` _locationx _locationy))
  (:`Started`
    (`self.ResetArmyDirector`)
    (bind _outhit (`KismetSystemLibrary.LineTraceSingle` _worldlocation (+ _worldlocation (* _worlddirection 1000.0)) "TraceTypeQuery1"))
    (bind (_bblockinghit _binitialoverlap _time _distance _location _impactpoint _normal _impactnormal _physmat _hitactor) (`GameplayStatics.BreakHitResult` _outhit))
    (bind (_asbp_land _bsuccess) (cast `/Game/Invade/Blueprints/BP_Land` _hitactor :!pure true))
    (if (and _bblockinghit _bsuccess)
      (set `self.isLandSelection` true)
      (bind _player_exists (`self.CheckIfLandContainsPlayer` _asbp_land))
      (if _player_exists
        (`KismetSystemLibrary.PrintString` "Selecting land")
        (else
          (`KismetSystemLibrary.PrintString` "Not your land to select")))))
  (:`Canceled`
    (`self.ResetArmyDirector` :!label _label))
  (:`Completed`
    (goto _label)))

(fn `CheckIfLandContainsPlayer`
  (params (`Land ref` :type "/Game/Invade/Blueprints/BP_Land Object Reference"))
  (returns (`Player Exists` :type Boolean))
  (bind _asps_player (cast `/Game/Invade/Blueprints/Managers/PS_Player` (`self.PlayerState`)))
  (for _array_element (`/Game/Invade/Blueprints/BP_Land.Armies` `Land ref`)
    (if (== (break `/Game/Invade/Blueprints/Structures/STRUCT_Army` _array_element) (`/Game/Invade/Blueprints/Managers/PS_Player.PlayerIndex` _asps_player))
      (return true)))
  (return false))

(fn `ResetArmyDirector`
  (`/Engine/EditorBlueprintResources/StandardMacros.IsValid` (`self.ArmyDirectorActor`)
    (:`Is Valid`
      _)
    (:`Is Not Valid`
      (bind _returnvalue (`|SpawnActorFromClass` :`Class` "/Game/Invade/Blueprints/BP_ArmyDirector.BP_ArmyDirector_C" :`SpawnTransform` (`KismetMathLibrary.MakeTransform` (0.0 0.0 0.0)) :`CollisionHandlingOverride` "AlwaysSpawn" :`TransformScaleMethod` "MultiplyWithRoot" :`Instigator` null))
      (set `self.ArmyDirectorActor` _returnvalue)))
  (`KismetArrayLibrary.Array_Clear` (`/Game/Invade/Blueprints/BP_ArmyDirector.LandRef` (`self.ArmyDirectorActor`))))

(fn `UserConstructionScript`)