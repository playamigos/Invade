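; GM_Main is the game mode that seeds the map's lands with armies and gives each joining player a starting land.
; On BeginPlay it gathers every BP_Land as unoccupied and adds a random-sized army to each.
; PostLogin moves a random land to the occupied list and overwrites its army entry with a larger one owned by the new player.
; It then stores the player index and starting land on PS_Player.
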(event `self.ReceiveBeginPlay`
  (bind _outactors (`GameplayStatics.GetAllActorsOfClass` "/Game/Invade/Blueprints/BP_Land.BP_Land_C"))
  (set `self.NonOccupiedLands` _outactors)
  (`self.GenerateInitArmiesOnLands`))

(event `self.K2_PostLogin`
  (params (NewPlayer :type "PlayerController Object Reference"))
  (bind _occupiedlands (`self.OccupiedLands`))
  (bind _occupiedlands_2 (`self.OccupiedLands`))
  (bind _output (`|GetArrayItem` _occupiedlands_2 (`KismetArrayLibrary.Array_LastIndex` _occupiedlands_2)))
  (set `self.NumOfPlayers` (+ (`self.NumOfPlayers`) 1))
  (`KismetArrayLibrary.Array_AddUnique` (`self.OccupiedLands`) (`KismetArrayLibrary.Array_Random` (`self.NonOccupiedLands`)))
  (`KismetArrayLibrary.Array_RemoveItem` (`self.NonOccupiedLands`) _output)
  (`KismetArrayLibrary.Array_Set` (`/Game/Invade/Blueprints/BP_Land.Armies` _output) 0 (make `/Game/Invade/Blueprints/Structures/STRUCT_Army` (`self.NumOfPlayers`) (`KismetMathLibrary.RandomIntegerInRange` 200 250)))
  (bind _asps_player (cast `/Game/Invade/Blueprints/Managers/PS_Player` (`Controller.PlayerState` NewPlayer)))
  (set `/Game/Invade/Blueprints/Managers/PS_Player.PlayerIndex` (`self.NumOfPlayers`) _asps_player)
  (set `/Game/Invade/Blueprints/Managers/PS_Player.StartingLand` (`|GetArrayItem` _occupiedlands (`KismetArrayLibrary.Array_LastIndex` _occupiedlands)) _asps_player))

(fn `GenerateInitArmiesOnLands`
  (for _array_element (`self.NonOccupiedLands`)
    (`KismetArrayLibrary.Array_Add` (`/Game/Invade/Blueprints/BP_Land.Armies` _array_element) (make `/Game/Invade/Blueprints/Structures/STRUCT_Army` 1 (`KismetMathLibrary.RandomIntegerInRange` 50 100)))))

(fn `UserConstructionScript`)