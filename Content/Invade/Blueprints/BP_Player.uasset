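; BP_Player is the player pawn that orbits the world origin in response to mouse drags, always facing the center.
; A tap starts rotation only when its cursor trace hits something other than BP_Land.
; While held, Tick adds mouse deltas to a target rotation, with pitch clamped and yaw free.
; Each frame it lerps toward that rotation and places itself at an eased TargetDistance behind its forward vector.
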(event `self.ReceiveBeginPlay`
  (set `PlayerController.bShowMouseCursor` true (`GameplayStatics.GetPlayerController` 0))
  (bind _asplayer_controller (cast `PlayerController` (`self.GetController`)))
  (`EnhancedInputSubsystemInterface.AddMappingContext` (pcsubsystem `EnhancedInputLocalPlayerSubsystem` _asplayer_controller) "/Game/Invade/Input/IMC_Main.IMC_Main" 0 (struct)))

(event `EnhancedInput|/Game/Invade/Input/Actions/IA_MouseTap`
  (params (ActionValue :type Boolean) (ElapsedSeconds :type "Float (double-precision)") (TriggeredSeconds :type "Float (double-precision)") (InputAction :type "InputAction Object Reference" :default "/Game/Invade/Input/Actions/IA_MouseTap.IA_MouseTap"))
  (bind _returnvalue (`GameplayStatics.GetPlayerController` 0))
  (bind (_locationx _locationy) (`PlayerController.GetMousePosition` _returnvalue))
  (bind (_worldlocation _worlddirection) (`PlayerController.DeprojectScreenPositionToWorld` _returnvalue _locationx _locationy))
  (:`Started`
    (set `self.PrevMousePosition` (`KismetMathLibrary.MakeVector` _locationx _locationy))
    (bind _outhit (`KismetSystemLibrary.LineTraceSingle` :`Start` _worldlocation :`End` (* _worlddirection 1000.0) :`TraceChannel` "TraceTypeQuery1" :`DrawDebugType` "Persistent"))
    (bind (_bblockinghit _binitialoverlap _time _distance _location _impactpoint _normal _impactnormal _physmat _hitactor) (`GameplayStatics.BreakHitResult` _outhit))
    (if (and _bblockinghit (not (`.bSuccess` (cast `/Game/Invade/Blueprints/BP_Land` _hitactor :!pure true))))
      (set `self.isRotatingView` true)
      (set `self.TargetRotation` (`self.K2_GetActorRotation`))))
  (:`Canceled`
    (set `self.isRotatingView` false :!label _label))
  (:`Completed`
    (goto _label)))

(event `self.ReceiveTick`
  (params (DeltaSeconds :type "Float (single-precision)"))
  (bind (_locationx _locationy) (`PlayerController.GetMousePosition` (`GameplayStatics.GetPlayerController` 0)))
  (`|ExecutionSequence`
    (:`then_0`
      (if (`self.isRotatingView`)
        (bind _output_get (set `self.CurrentMouseposition` (`KismetMathLibrary.MakeVector` _locationx _locationy)))
        (bind (_returnvalue_x _returnvalue_y) (`KismetMathLibrary.BreakVector` (* (- _output_get (`self.PrevMousePosition`)) (1.0 -1.0 0.0))))
        (`self.SetTargetRotation` true (`KismetMathLibrary.MakeRotator` 0.0 _returnvalue_y _returnvalue_x))
        (set `self.PrevMousePosition` (`self.CurrentMouseposition`))))
    (:`then_1`
      (`self.UpdatePlayerTransform` DeltaSeconds))))

(fn `ClampPitch`
  (params (pitch :type "Float (double-precision)"))
  (returns (`clamped pitch` :type "Float (double-precision)"))
  (return (`KismetMathLibrary.ClampAngle` pitch -85.0 85.0)))

(fn `ClampYaw`
  (params (yaw :type "Float (double-precision)"))
  (returns (`clamped jaw` :type "Float (double-precision)"))
  (return yaw))

(fn `SetTargetRotation`
  (params (isDiff :type Boolean) (rot :type "Rotator Structure"))
  (bind (_rot_roll _rot_pitch _rot_yaw) (`KismetMathLibrary.BreakRotator` (`local.rot`)))
  (bind (_rot_roll_2 _rot_pitch_2 _rot_yaw_2) (`KismetMathLibrary.BreakRotator` (`local.rot`)))
  (bind (_targetrotation_roll _targetrotation_pitch _targetrotation_yaw) (`KismetMathLibrary.BreakRotator` (`self.TargetRotation`)))
  (if isDiff
    (set `self.TargetRotation` (`KismetMathLibrary.MakeRotator` 0.0 (`self.ClampPitch` (+ _targetrotation_pitch _rot_pitch_2)) (`self.ClampYaw` (+ _targetrotation_yaw _rot_yaw_2))))
    (else
      (set `self.TargetRotation` (`KismetMathLibrary.MakeRotator` 0.0 (`self.ClampPitch` _rot_pitch) (`self.ClampYaw` _rot_yaw))))))

(fn `UpdatePlayerTransform`
  (params (DeltaSeconds :type "Float (double-precision)"))
  (bind (_returnvalue_roll _returnvalue_pitch _returnvalue_yaw) (`KismetMathLibrary.BreakRotator` (`self.K2_GetActorRotation`)))
  (bind (_targetrotation_roll _targetrotation_pitch _targetrotation_yaw) (`KismetMathLibrary.BreakRotator` (`self.TargetRotation`)))
  (bind _returnvalue (* DeltaSeconds (`self.speed`)))
  (`self.K2_SetActorRotation` (`KismetMathLibrary.RLerp` (`KismetMathLibrary.MakeRotator` 0.0 _returnvalue_pitch _returnvalue_yaw) (`KismetMathLibrary.MakeRotator` 0.0 _targetrotation_pitch _targetrotation_yaw) _returnvalue))
  (`self.K2_SetActorLocation` (* (`self.GetActorForwardVector`) (`KismetMathLibrary.Lerp` (`KismetMathLibrary.VSize` (`self.K2_GetActorLocation`)) (`self.TargetDistance`) _returnvalue) -1.0)))

(fn `UserConstructionScript`)