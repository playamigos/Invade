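; BP_Land is a land actor that places itself on the surface of an origin-centred sphere with a fixed radius.
; The construction script converts the PlacementYaw and PlacementPitch angles into a spherical position, then sets the world location with local Z pointing outward from the centre.
; The event graph holds only disabled default events, so the Blueprint has no runtime logic.
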(fn `UserConstructionScript`
  (bind _placementyaw (`self.PlacementYaw`))
  (bind _placementpitch (`self.PlacementPitch`))
  (bind _returnvalue (`KismetMathLibrary.DegCos` _placementpitch))
  (bind _returnvalue_2 (* (`KismetMathLibrary.MakeVector` (* (`KismetMathLibrary.DegCos` _placementyaw) _returnvalue) (* (`KismetMathLibrary.DegSin` _placementyaw) _returnvalue) (`KismetMathLibrary.DegSin` _placementpitch)) 250.0))
  (`self.K2_SetActorLocationAndRotation` _returnvalue_2 (`KismetMathLibrary.MakeRotFromZ` _returnvalue_2)))